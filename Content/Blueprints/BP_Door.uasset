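; BP_Door is a door that slides open for a BP_BasicPlayer whose Collected count is above zero.
; Box begin and end overlaps share that check and play the DoorMove timeline, which adds a lerped sideways offset to DoorMesh each update, so movement accumulates.
; The construction script sets DoorText from DoorString.
; The DoorBack return timeline and alternate text setters are unconnected, so nothing closes the door.
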(event OnComponentBeginOverlap(Box)
  (params (OverlappedComponent :type Primitive%20Component%20Object%20Reference) (OtherActor :type Actor%20Object%20Reference) (OtherComp :type Primitive%20Component%20Object%20Reference) (OtherBodyIndex :type Integer) (bFromSweep :type Boolean) (SweepResult :type Hit%20Result%20Structure%20%28by%20ref%29))
  (bind _asbp_basic_player (Utilities|Casting|CastToBP_BasicPlayer OtherActor))
  (if (> (Variables|/Game/Blueprints/BP_BasicPlayer.BP_BasicPlayer_C|GetCollected _asbp_basic_player) 0)
    (bind _alpha (Timeline|DoorMove Play)
      (:Update
        (Transformation|AddRelativeLocation (Variables|Default|GetDoor_Mesh) (Math|Vector|Lerp(Vector) "0, 0, 0" "0.000000,4.000000, 0" _alpha) false false)))))

(event OnComponentEndOverlap(Box)
  (params (OverlappedComponent :type Primitive%20Component%20Object%20Reference) (OtherActor :type Actor%20Object%20Reference) (OtherComp :type Primitive%20Component%20Object%20Reference) (OtherBodyIndex :type Integer))
  (Utilities|Casting|CastToBP_BasicPlayer OtherActor)
  (if (> (Variables|/Game/Blueprints/BP_BasicPlayer.BP_BasicPlayer_C|GetCollected (stale OnComponentBeginOverlap(Box) _asbp_basic_player)) 0)
    (bind _alpha (Timeline|DoorMove Play)
      (:Update
        (Transformation|AddRelativeLocation (Variables|Default|GetDoor_Mesh) (Math|Vector|Lerp(Vector) "0, 0, 0" "0.000000,4.000000, 0" _alpha) false false)))))

(fn ConstructionScript
  (Rendering|Components|TextRender|SetText (Variables|Default|GetDoor_Text) (Utilities|Text|ToText(String) (Variables|Default|GetDoorString))))