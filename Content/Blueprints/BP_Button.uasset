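; BP_Button is a toggle button that switches linked platforms, a light and a door on and off.
; Each Activated_Door call alternates through a FlipFlop, playing an on or off sound at the button and swapping its material.
; The on press starts both platforms, lights the point light and opens the door; the next press stops the platforms, zeroes the light intensity and closes the door.
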(event Custom|Activated_Door
  (bind _buttom (Variables|Default|GetButtom))
  (bind _doormesh (Variables|Default|GetDoorMesh))
  (bind _platform_1 (Variables|Default|GetPlatform_1))
  (bind _light (Variables|Default|GetLight))
  ;[1 1 1] Button Pressed
  (Utilities|FlowControl|FlipFlop
    (:A
      (Audio|PlaySoundatLocation "/Game/Sounds/243038__testing-player__button.243038__testing-player__button" (Transformation|GetWorldLocation (Variables|Default|GetButtom)) "0, 0, 0" 1.0 1.0 0.0 0 0 0)
      (Rendering|Material|SetMaterial _buttom 0 "/Game/Materials/Stair_Stone.Stair_Stone")
      (Default|StartPlatform _platform_1)
      (Rendering|Components|Light|SetIntensity (Variables|/Script/Engine.PointLight|GetPointLightComponent _light) 1e+01)
      (Default|OpenDoor _doormesh))
    (:B
      (Audio|PlaySoundatLocation "/Game/Sounds/63528__florian-reinke__button-off.63528__florian-reinke__button-off" (Transformation|GetWorldLocation (Variables|Default|GetButtom)) "0, 0, 0" 1.0 1.0 0.0 0 0 0)
      (Rendering|Material|SetMaterial _buttom 0 "/Game/Materials/Door_Color.Door_Color")
      (Default|StopPlatform _platform_1)
      (Rendering|Components|Light|SetIntensity (Variables|/Script/Engine.PointLight|GetPointLightComponent _light) 0.0)
      (Default|CloseDoor _doormesh))))

(fn ConstructionScript)