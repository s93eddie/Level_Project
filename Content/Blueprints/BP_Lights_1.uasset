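; BP_Lights_1 is a light made of a sphere mesh and a point light that can turn on and change color.
; LightTurnOn waits for the Time delay, swaps the sphere's material, then uses a timeline to ramp the point light from zero to its Intensity.
; ChangeLightColor swaps to another material and uses a second timeline to blend the light from warm yellow to light blue.
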(event Custom|Light%20Turn%20On
  (Utilities|FlowControl|Delay (Variables|Default|GetTime))
  (Rendering|Material|SetMaterial (Variables|Default|GetSphere) 0 "/Game/Materials/Light_1.Light_1")
  (bind _newtrack_0 (Timeline|Timeline_0 Play)
    (:Update
      (Rendering|Components|Light|SetIntensity (Variables|Default|GetPointLight) (Math|Float|Lerp 0.0 (Variables|Default|GetIntensity) _newtrack_0)))))

(event Custom|Change%20Light%20Color
  (Rendering|Material|SetMaterial (Variables|Default|GetSphere) 0 "/Game/Materials/Light_3.Light_3")
  (bind _color_time (Timeline|Change%20Color Play)
    (:Update
      (Rendering|Components|Light|SetLightColor (Variables|Default|GetPointLight) (Math|Color|Lerp(LinearColor) "(R=1.000000,G=0.854993,B=0.564712,A=1.000000)" "(R=0.332452,G=0.791298,B=1.000000,A=1.000000)" _color_time) true))))

(fn ConstructionScript)