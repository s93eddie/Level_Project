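; BP_Outer_Light is an outer light fixture that switches on when its OuterLightTurnOn event fires.
; After a short delay, it swaps the materials on three spheres, with the middle one differing from the outer two.
; Three timelines then ramp three point lights up from zero intensity.
; Each timeline starts the next from its Update pin rather than Finished, so the fades overlap instead of running sequentially.
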(event Custom|Outer%20Light%20Turn%20On
  (Utilities|FlowControl|Delay 0.3)
  (Rendering|Material|SetMaterial (Variables|Default|GetSphere%201) 0 "/Game/Materials/Light_1.Light_1")
  (Rendering|Material|SetMaterial (Variables|Default|GetSphere%202) 0 "/Game/Materials/Light_2.Light_2")
  (Rendering|Material|SetMaterial (Variables|Default|GetSphere%203) 0 "/Game/Materials/Light_1.Light_1")
  (bind _newtrack_0 (Timeline|Outer%20Light Play)
    (:Update
      (Rendering|Components|Light|SetIntensity (Variables|Default|GetPointLight%201) (Math|Float|Lerp 0.0 1.55e+03 _newtrack_0))
      (bind _newtrack_0_2 (Timeline|Timeline_0 Play)
        (:Update
          (Rendering|Components|Light|SetIntensity (Variables|Default|GetPointLight%202) (Math|Float|Lerp 0.0 1.5e+03 _newtrack_0_2))
          (bind _newtrack_0_3 (Timeline|Timeline_1 Play)
            (:Update
              (Rendering|Components|Light|SetIntensity (Variables|Default|GetPointLight%203) (Math|Float|Lerp 0.0 1.6e+03 _newtrack_0_3)))))))))

(fn ConstructionScript)