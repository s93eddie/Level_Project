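; BP_Door is a sliding door that opens for a BP_BasicPlayer whose Collected count is above zero.
; The DoorMove timeline lerps DoorMeshHandle sideways along local Y, playing on box overlap and reversing when the overlap ends.
; OpenDoor and CloseDoor events drive the same timeline without that check.
; The construction script fills DoorText from DoorString, while two other text setters are left unconnected.
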(event OnComponentBeginOverlap(Box)
  (params (OverlappedComponent :type Primitive%20Component%20Object%20Reference) (OtherActor :type Actor%20Object%20Reference) (OtherComp :type Primitive%20Component%20Object%20Reference) (OtherBodyIndex :type Integer) (bFromSweep :type Boolean) (SweepResult :type Hit%20Result%20Structure%20%28by%20ref%29))
  ;[1 1 1] Door Open & Close
  (bind _asbp_basic_player (Utilities|Casting|CastToBP_BasicPlayer OtherActor))
  (if (> (Variables|/Game/Blueprints/BP_BasicPlayer.BP_BasicPlayer_C|GetCollected _asbp_basic_player) 0)
    (bind _alpha (Timeline|DoorMove Play)
      (:Update
        (Transformation|SetRelativeLocation (Variables|Default|GetDoorMeshHandle) (Math|Vector|Lerp(Vector) "0, 0, 0" "0.000000,200.000000,0.000000" _alpha) false false)))))

(event OnComponentEndOverlap(Box)
  (params (OverlappedComponent :type Primitive%20Component%20Object%20Reference) (OtherActor :type Actor%20Object%20Reference) (OtherComp :type Primitive%20Component%20Object%20Reference) (OtherBodyIndex :type Integer))
  ;[1 1 1] Door Open & Close
  (Utilities|Casting|CastToBP_BasicPlayer OtherActor)
  (if (> (Variables|/Game/Blueprints/BP_BasicPlayer.BP_BasicPlayer_C|GetCollected (stale OnComponentBeginOverlap(Box) _asbp_basic_player)) 0)
    (bind _alpha (Timeline|DoorMove Reverse)
      (:Update
        (Transformation|SetRelativeLocation (Variables|Default|GetDoorMeshHandle) (Math|Vector|Lerp(Vector) "0, 0, 0" "0.000000,200.000000,0.000000" _alpha) false false)))))

(event Custom|Open%20Door
  ;[1 1 1] Door Open & Close
  (bind _alpha (Timeline|DoorMove Play)
    (:Update
      (Transformation|SetRelativeLocation (Variables|Default|GetDoorMeshHandle) (Math|Vector|Lerp(Vector) "0, 0, 0" "0.000000,200.000000,0.000000" _alpha) false false))))

(event Custom|Close%20Door
  ;[1 1 1] Door Open & Close
  (bind _alpha (Timeline|DoorMove Reverse)
    (:Update
      (Transformation|SetRelativeLocation (Variables|Default|GetDoorMeshHandle) (Math|Vector|Lerp(Vector) "0, 0, 0" "0.000000,200.000000,0.000000" _alpha) false false))))

(fn ConstructionScript
  (Rendering|Components|TextRender|SetText (Variables|Default|GetDoor_Text) (Utilities|Text|ToText(String) (Variables|Default|GetDoorString))))