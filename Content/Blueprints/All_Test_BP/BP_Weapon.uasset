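; BP_Weapon is an auto-firing turret that shows a dialogue widget when a player is nearby.
; A timeline started at BeginPlay moves the cylinder along Y, and its Fire event spawns a scaled BP_Projectile at the arrow.
; Both Fire and Finished lead into a shared delay that restarts the timeline.
; Box overlap with BP_BasicPlayer toggles Occupid and adds or removes BP_Dialogue, without affecting firing.
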(event OnComponentBeginOverlap(Box)
  (params (OverlappedComponent :type Primitive%20Component%20Object%20Reference) (OtherActor :type Actor%20Object%20Reference) (OtherComp :type Primitive%20Component%20Object%20Reference) (OtherBodyIndex :type Integer) (bFromSweep :type Boolean) (SweepResult :type Hit%20Result%20Structure%20%28by%20ref%29))
  (Utilities|Casting|CastToBP_BasicPlayer OtherActor)
  (Variables|Default|SetOccupid true)
  (bind _returnvalue (UserInterface|CreateWidget "/Game/Blueprints/All_UI_BP/BP_Dialogue.BP_Dialogue_C"))
  (bind _output_get (Variables|Default|SetDialogue _returnvalue))
  (UserInterface|Viewport|AddtoViewport _output_get 0))

(event OnComponentEndOverlap(Box)
  (params (OverlappedComponent :type Primitive%20Component%20Object%20Reference) (OtherActor :type Actor%20Object%20Reference) (OtherComp :type Primitive%20Component%20Object%20Reference) (OtherBodyIndex :type Integer))
  (Utilities|Casting|CastToBP_BasicPlayer OtherActor)
  (Variables|Default|SetOccupid false)
  (Widget|RemovefromParent (Variables|Default|GetDialogue)))

(event EventBeginPlay
  (bind _arrow (Variables|Default|GetArrow))
  (bind _turrentfire (Timeline|Timeline_0 PlayFromStart)
    (:Update
      (Transformation|SetRelativeLocation (Variables|Default|GetCylinder) (Math|Vector|MakeVector 0.0 _turrentfire 0.0) false false))
    (:Finished
      (Utilities|FlowControl|Delay (Variables|Default|GetDelayTime) :!label _label)
      (Timeline|Timeline_0 PlayFromStart))
    (:Fire
      (Game|SpawnActorfromClass "/Game/Blueprints/All_Test_BP/BP_Projectile.BP_Projectile_C" (Math|Transform|MakeTransform (Transformation|GetWorldLocation _arrow) (Transformation|GetWorldRotation _arrow) (Math|Conversions|ToVector(Float) (Variables|Default|GetProjectileScale))) "AlwaysSpawn" 0 0)
      (goto _label))))

(fn ConstructionScript)