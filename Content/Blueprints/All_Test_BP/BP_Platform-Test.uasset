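; Test moving platform that shuttles back and forth between StartPoint and EndPoint once StartPlatform is called.
; A timeline lerps the relative location of PlatformHandle, and on each finish a short delay feeds a FlipFlop that alternates reverse and play.
; StopPlatform stops the timeline, and the construction script places the handle at StartPoint.
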(event Custom|StartPlatform
  (bind _alpha (Timeline|Platorm Play)
    (:Update
      (Transformation|SetRelativeLocation (Variables|Default|GetPlatformHandle) (Math|Vector|Lerp(Vector) (Variables|Default|GetStartPoint) (Variables|Default|GetEndPoint) _alpha) false false))
    (:Finished
      (Utilities|FlowControl|Delay 0.5)
      (Utilities|FlowControl|FlipFlop
        (:A
          (Timeline|Platorm Reverse))
        (:B
          (Timeline|Platorm Play))))))

(event Custom|StopPlatform
  (bind _alpha (Timeline|Platorm Stop)
    (:Update
      (Transformation|SetRelativeLocation (Variables|Default|GetPlatformHandle) (Math|Vector|Lerp(Vector) (Variables|Default|GetStartPoint) (Variables|Default|GetEndPoint) _alpha) false false))
    (:Finished
      (Utilities|FlowControl|Delay 0.5)
      (Utilities|FlowControl|FlipFlop
        (:A
          (Timeline|Platorm Reverse))
        (:B
          (Timeline|Platorm Play))))))

(fn ConstructionScript
  (Transformation|SetRelativeLocation (Variables|Default|GetPlatformHandle) (Variables|Default|GetStartPoint) false false))